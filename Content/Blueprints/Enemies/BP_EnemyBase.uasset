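; BP_EnemyBase is an enemy base Blueprint that tracks health and death.
; The construction script sets current health to the maximum, and AnyDamage subtracts incoming damage, clamped between zero and that maximum.
; When health first reaches zero, it sets a dead flag so EnemyDied is called only once.
; EnemyDied is empty here, so this Blueprint defines no death behavior of its own.
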(event `self.ReceiveAnyDamage`
  (params (Damage :type "Float (single-precision)") (DamageType :type "DamageType Object Reference") (InstigatedBy :type "Controller Object Reference") (DamageCauser :type "Actor Object Reference"))
  (set `self.CurrentHealth` (`KismetMathLibrary.FClamp` (- (`self.CurrentHealth`) Damage) 0.0 (`self.MaxHealth`)))
  (if (and (<= (`self.CurrentHealth`) 0.0) (not (`self.BisDead`)))
    (set `self.BisDead` true)
    (`self.EnemyDied`)))

(fn `EnemyDied`)

(fn `UserConstructionScript`
  (set `self.CurrentHealth` (`self.MaxHealth`)))