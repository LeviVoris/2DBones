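; BP_InteractiveHealth is an interactive health pickup that heals the hero who uses it.
; Interact checks the hero's current health against a hardcoded full-health threshold, adds HealthValue through AddHealth when below it, then destroys the pickup.
; At full health the interaction does nothing, so the pickup stays in the world.
; All logic lives in Interact, as the event graph holds only disabled default events.
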(fn `Interact`
  (params (HeroRef :type "/Game/Blueprints/BP_HeroBase Object Reference"))
  (if (not (>= (`/Game/Blueprints/BP_HeroBase.CurrentHealth` (`local.HeroRef`)) 100.0))
    (`/Game/Blueprints/BP_HeroBase.AddHealth` (`local.HeroRef`) (`self.HealthValue`))
    (`self.K2_DestroyActor`)))

(fn `UserConstructionScript`
  (`parent.UserConstructionScript`))